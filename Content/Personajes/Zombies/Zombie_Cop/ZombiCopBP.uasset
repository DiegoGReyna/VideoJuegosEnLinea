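; Zombie cop enemy character that hunts the player by sight and sound, punches in melee and dies when its health runs out.
; PawnSensing drives AIMoveTo, re-issued on a short retriggerable delay while chasing, and plays a punch montage on arrival.
; The Ataque event sphere-traces at the right-hand socket to deal damage.
; MakeDamage handles health and death, while Tick updates a health-bar widget that yaws toward the camera.
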(event `self.PawnSensing.OnHearNoise`
  (params (Instigator :type "Pawn Object Reference") (Location :type "Vector Structure (by ref)") (Volume :type "Float (single-precision)"))
  ;[1 1 1] Inteligencia Artificial
  (if (not (`AnimInstance.IsAnyMontagePlaying` (`SkeletalMeshComponent.GetAnimInstance` (`self.Mesh`))))
    (`|AIMoveTo` self Location null 10.0)))

(event `self.PawnSensing.OnSeePawn`
  (params (Pawn :type "Pawn Object Reference"))
  (bind _returnvalue (`AnimInstance.IsAnyMontagePlaying` (`SkeletalMeshComponent.GetAnimInstance` (`self.Mesh`))))
  ;[1 1 1] Inteligencia Artificial
  (bind _asue_4asp_character (cast `/Game/AnimStarterPack/Ue4ASP_Character` Pawn :!label _label))
  (if (not _returnvalue)
    (`|AIMoveTo` self (0.0 0.0 0.0) _asue_4asp_character 10.0
      (:`then`
        (`KismetSystemLibrary.RetriggerableDelay` 0.1)
        (goto _label))
      (:`OnSuccess`
        (if (not _returnvalue)
          (`|PlayMontage` (`self.Mesh`) "/Game/Personajes/Zombies/ZombieAnimations/ZombieCop_Punch.ZombieCop_Punch"
            (:`then`
              (`GameplayStatics.PlaySoundAtLocation` "/Game/Audio/ZombieAttack.ZombieAttack" (`self.K2_GetActorLocation`) (struct) 1.0 1.0 0.0 null null null null))))))))

(event `self.ReceiveTick`
  (params (DeltaSeconds :type "Float (single-precision)"))
  ;[1 1 1] Salud_Enemigo
  (bind _assalud_enemigo (cast `/Game/Personajes/Zombies/Zombie_Cop/SaludEnemigo` (`WidgetComponent.GetUserWidgetObject` (`self.Salud`))))
  (`ProgressBar.SetPercent` (`/Game/Personajes/Zombies/Zombie_Cop/SaludEnemigo.ProgressBar_65` _assalud_enemigo) (/ (`self.Health`) 200.0))
  (`SceneComponent.K2_SetWorldRotation` (`self.Salud`) (`KismetMathLibrary.MakeRotator` 0.0 0.0 (.yaw (`KismetMathLibrary.FindLookAtRotation` (`SceneComponent.K2_GetComponentLocation` (`self.Salud`)) (`self.K2_GetActorLocation` (`GameplayStatics.GetPlayerCameraManager` 0))))) false false))

(event `Ataque`
  (bind _returnvalue (`SceneComponent.GetSocketLocation` (`self.Mesh`) "RightHand"))
  ;[1 1 1] Generar Daño
  (bind (_outhit _returnvalue_2) (`KismetSystemLibrary.SphereTraceSingle` :`Start` _returnvalue :`End` _returnvalue :`Radius` 80.0 :`TraceChannel` "TraceTypeQuery2" :`TraceColor` (struct :`R` 1.0) :`TraceHitColor` (struct :`G` 1.0)))
  (if _returnvalue_2
    (bind (_bblockinghit _binitialoverlap _time _distance _location _impactpoint _normal _impactnormal _physmat _hitactor) (`GameplayStatics.BreakHitResult` _outhit))
    (`GameplayStatics.ApplyDamage` _hitactor 20.0 (`self.GetInstigatorController` _hitactor) self)
    (bind _asue_4asp_character (cast `/Game/AnimStarterPack/Ue4ASP_Character` _hitactor))
    (`/Game/AnimStarterPack/Ue4ASP_Character.Atacked` _asue_4asp_character)))

(event `MakeDamage`
  (params (Damage :type "Float (double-precision)" :default 10.0))
  ;[1 1 1] Recibir_Daño
  (if (not (<= (`self.Health`) 0.0))
    (bind _output_get (set `self.Health` (- (`self.Health`) Damage)))
    (if (<= _output_get 0.0)
      (`SkeletalMeshComponent.PlayAnimation` (`self.Mesh`) (`self.ZombieCopDeath`) false)
      (`SceneComponent.SetVisibility` (`self.Salud`) false false)
      (`self.DetachFromControllerPendingDestroy`)
      (`KismetSystemLibrary.Delay` 4.0)
      (`self.K2_DestroyActor`))))

(fn `UserConstructionScript`)