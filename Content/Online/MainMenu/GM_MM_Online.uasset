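; Game mode for the online main menu that tracks connected player controllers and provides spawning for menu characters.
; Login and controller swaps add controllers to AllPC, while logout removes those that cast to PC_MM_Online.
; SpawnPlayer, not called within this graph, destroys any existing pawn, spawns a MainMenuCharacter and possesses it.
; FindTransform supplies the spawn location by picking a random PlayerStart.
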(event `self.K2_PostLogin`
  (params (NewPlayer :type "PlayerController Object Reference"))
  ;[1 1 1] OnLogin
  (`KismetArrayLibrary.Array_Add` (`self.AllPC`) NewPlayer))

(event `self.K2_OnSwapPlayerControllers`
  (params (OldPC :type "PlayerController Object Reference") (NewPC :type "PlayerController Object Reference"))
  ;[1 1 1] OnLogin
  (`KismetArrayLibrary.Array_Add` (`self.AllPC`) NewPC))

(event `self.K2_OnLogout`
  (params (ExitingController :type "Controller Object Reference"))
  ;[1 1 1] LogOut
  (bind _aspc_mm_online (cast `/Game/Online/MainMenu/PC_MM_Online` ExitingController))
  (`KismetArrayLibrary.Array_RemoveItem` (`self.AllPC`) _aspc_mm_online))

(fn `Find_Transform`
  (returns (PositionTransform :type "Transform Structure"))
  (bind _outactors (`GameplayStatics.GetAllActorsOfClass` "/Script/Engine.PlayerStart"))
  (return (`self.GetTransform` (`|GetArrayItem` _outactors (`KismetMathLibrary.RandomIntegerInRange` (- (`KismetArrayLibrary.Array_Length` _outactors) 1))))))

(fn `SpawnPlayer`
  (params (PlayerController :type "PlayerController Object Reference"))
  (bind _returnvalue (`Controller.K2_GetPawn` PlayerController))
  (`/Engine/EditorBlueprintResources/StandardMacros.IsValid` _returnvalue
    (:`Is Valid`
      (`self.K2_DestroyActor` _returnvalue))
    (:`Is Not Valid`
      _))
  (bind _returnvalue_2 (`|SpawnActorFromClass` "/Game/MENU/MainMenuCharacter.MainMenuCharacter_C" (`self.Find_Transform`) "Undefined" "OverrideRootScale" null null))
  (`Controller.Possess` PlayerController _returnvalue_2))

(fn `UserConstructionScript`)