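; Online game mode for the hangar level that tracks connected player controllers and spawns their characters.
; Post-login and controller swaps add to the AllPCs array, and logout removes online controllers from it.
; SpawnPlayer destroys the existing pawn and spawns an Ue4ASP_Character at a random PlayerStart.
; The array's last index, not the controller's own, selects one of four meshes before possession, with no case beyond four players.
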(event `self.K2_PostLogin`
  (params (NewPlayer :type "PlayerController Object Reference"))
  ;[1 1 1] Login
  (`KismetArrayLibrary.Array_Add` (`self.All_PCs`) NewPlayer))

(event `self.K2_OnSwapPlayerControllers`
  (params (OldPC :type "PlayerController Object Reference") (NewPC :type "PlayerController Object Reference"))
  ;[1 1 1] Login
  (`KismetArrayLibrary.Array_Add` (`self.All_PCs`) NewPC))

(event `self.K2_OnLogout`
  (params (ExitingController :type "Controller Object Reference"))
  ;[1 1 1] Logout
  (bind _asbp_pc_online (cast `/Game/Online/HangarLevel/BP_PC_Online` ExitingController))
  (`KismetArrayLibrary.Array_RemoveItem` (`self.All_PCs`) _asbp_pc_online))

(fn `Find_Random_Player_Start`
  (returns (Player_Start_Transform :type "Transform Structure"))
  (bind _outactors (`GameplayStatics.GetAllActorsOfClass` "/Script/Engine.PlayerStart"))
  (return (`self.GetTransform` (`|GetArrayItem` _outactors (`KismetMathLibrary.RandomIntegerInRange` 0 (- (`KismetArrayLibrary.Array_Length` _outactors) 1))))))

(fn `Spawn_Player`
  (params (PlayerController :type "PlayerController Object Reference"))
  (bind _returnvalue (`Controller.K2_GetPawn` PlayerController))
  (`/Engine/EditorBlueprintResources/StandardMacros.IsValid` _returnvalue
    (:`Is Valid`
      (`self.K2_DestroyActor` _returnvalue))
    (:`Is Not Valid`
      _))
  (bind _returnvalue_2 (`|SpawnActorFromClass` "/Game/AnimStarterPack/Ue4ASP_Character.Ue4ASP_Character_C" (`self.Find_Random_Player_Start`) "Undefined" "OverrideRootScale" null null))
  (switch `int` (`KismetArrayLibrary.Array_LastIndex` (`self.All_PCs`))
    (:`0`
      (`/Game/AnimStarterPack/Ue4ASP_Character.SetMeshOnServer` _returnvalue_2 "/Game/Personajes/Humanos/Personaje01/Ch11_nonPBR.Ch11_nonPBR"))
    (:`1`
      (`/Game/AnimStarterPack/Ue4ASP_Character.SetMeshOnServer` _returnvalue_2 "/Game/PrincipalCharacter/PrincipalCharacter.PrincipalCharacter"))
    (:`2`
      (`/Game/AnimStarterPack/Ue4ASP_Character.SetMeshOnServer` _returnvalue_2 "/Game/Personajes/Humanos/personajes05/Ch15_nonPBR.Ch15_nonPBR"))
    (:`3`
      (`/Game/AnimStarterPack/Ue4ASP_Character.SetMeshOnServer` _returnvalue_2 "/Game/Personajes/Humanos/personajes04/Ch07_nonPBR.Ch07_nonPBR")))
  (`Controller.Possess` PlayerController _returnvalue_2))

(fn `UserConstructionScript`)